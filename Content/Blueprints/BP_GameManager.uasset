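; BP_GameManager scatters a batch of Arrow actors through the world when play begins.
; SpawnArrows loops on ArrowsToSpawn, deriving random X and Z from the player's viewport pixel size, used directly as world coordinates.
; ShouldNegate makes a coin flip intended to vary their sign, while Y lies between ArrowDepth and twice that depth.
; Spawning always succeeds regardless of collisions.
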(event `self.ReceiveBeginPlay`
  (`self.SpawnArrows`))

(fn `ShouldNegate`
  (params (In :type "Float (double-precision)"))
  (returns (Out :type "Float (double-precision)"))
  (locals (Input :type "Float (double-precision)"))
  (bind _output_get (set `local.Input` In))
  (if (== (`KismetMathLibrary.RandomIntegerInRange` 0 1) 0)
    (`/Engine/EditorBlueprintResources/StandardMacros.NegateFloat` _output_get
      (:`  `
        _)))
  (return (`local.Input`)))

(fn `SpawnArrows`
  (locals (xPos :type "Float (double-precision)") (yPos :type "Float (double-precision)") (zPos :type "Float (double-precision)"))
  (bind (_sizex _sizey) (`PlayerController.GetViewportSize` (`GameplayStatics.GetPlayerController` 0)))
  (for _ (range (+ (`self.ArrowsToSpawn`) 1))
    (bind _out (`self.ShouldNegate` (* _sizex (`KismetMathLibrary.RandomFloat`))))
    (set `local.xPos` _out)
    (bind _out_2 (`self.ShouldNegate` (* _sizey (`KismetMathLibrary.RandomFloat`))))
    (set `local.zPos` _out_2)
    (set `local.yPos` (+ (`self.ArrowDepth`) (* (`self.ArrowDepth`) (`KismetMathLibrary.RandomFloat`))))
    (`|SpawnActorFromClass` (`self.Arrow`) (`KismetMathLibrary.MakeTransform` (`KismetMathLibrary.MakeVector` (`local.xPos`) (`local.yPos`) (`local.zPos`))) "AlwaysSpawn" "OverrideRootScale" null null)))

(fn `UserConstructionScript`)